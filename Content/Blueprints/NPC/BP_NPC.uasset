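; NPC character that switches from idle/walk to chasing the first pawn it sees, feeding its AI controller's blackboard.
; BeginPlay writes roaming range and state to the blackboard through the GetBB helper, then sets walk speed by state.
; PawnSensing stores a seen pawn as Enemy when none is valid, then sets Chase and doubles walk speed.
; The Chase change stays on the actor; the blackboard's NPC_State is written only at BeginPlay.
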(event `self.ReceiveBeginPlay`
  (bind (_returnvalue _returnvalue1) (`self.Get_BB` "RoamingRange"))
  (bind (_returnvalue_2 _returnvalue1_2) (`self.Get_BB` "NPC_State"))
  (`BlackboardComponent.SetValueAsFloat` _returnvalue _returnvalue1 (`self.RoamingRange`))
  (`BlackboardComponent.SetValueAsEnum` _returnvalue_2 _returnvalue1_2 (`self.State`))
  (`self.SetWalkspeedByState`))

(event `self.PawnSensing.OnSeePawn`
  (params (Pawn :type "Pawn Object Reference"))
  (bind (_returnvalue _returnvalue1) (`self.Get_BB` "Enemy"))
  (`self.EnemyPawn`
    (:`then`)
    (:`else`
      (bind _output_get (set `self.EnemyPawn` Pawn))
      (`BlackboardComponent.SetValueAsObject` _returnvalue _returnvalue1 _output_get)
      (set `self.State` "NewEnumerator1")
      (`self.SetWalkspeedByState`))))

(fn `Get_BB`
  (params (Value :type Name))
  (returns (ReturnValue :type "BlackboardComponent Object Reference") (ReturnValue1 :type Name))
  (return (`AIBlueprintHelperLibrary.GetBlackboard` (`AIBlueprintHelperLibrary.GetAIController` self)) (`KismetSystemLibrary.MakeLiteralName` Value)))

(fn `SetWalkspeedByState`
  (bind _charactermovement (`self.CharacterMovement`))
  (switch `/Game/Blueprints/NPC/E_NPC_State` (`self.State`)
    (:`NewEnumerator0`
      (set `CharacterMovementComponent.MaxWalkSpeed` 100.0 _charactermovement))
    (:`NewEnumerator1`
      (set `CharacterMovementComponent.MaxWalkSpeed` 200.0 _charactermovement))))

(fn `UserConstructionScript`)