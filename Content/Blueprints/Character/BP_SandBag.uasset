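; BP_SandBag is an enemy pawn that chases pawns it sees and can be killed by damage.
; Its PawnSensing component triggers an AI MoveTo toward any seen pawn.
; AnyDamage feeds SetHealth, which subtracts damage, clamps Health between zero and its current value, and sets IsDead at zero, after which the actor destroys itself.
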(event `self.PawnSensing.OnSeePawn`
  (params (Pawn :type "Pawn Object Reference"))
  (`|AIMoveTo` self (0.0 0.0 0.0) Pawn))

(event `self.ReceiveAnyDamage`
  (params (Damage :type "Float (single-precision)") (DamageType :type "DamageType Object Reference") (InstigatedBy :type "Controller Object Reference") (DamageCauser :type "Actor Object Reference"))
  ;[1 1 1] 적 죽음
  (`self.SetHealth` Damage)
  (if (`self.bIsDead`)
    (`self.K2_DestroyActor`)))

(fn `SetHealth`
  (params (Damage :type "Float (double-precision)"))
  (bind _output_get (set `self.Health` (`KismetMathLibrary.FClamp` (- (`self.Health`) Damage) 0.0 (`self.Health`))))
  (if (== _output_get 0.0)
    (set `self.bIsDead` true)))

(fn `UserConstructionScript`)