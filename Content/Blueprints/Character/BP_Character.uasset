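; Player character with movement, interaction, melee combat, two weapon slots, HP with delayed respawn, and EXP leveling.
; BeginPlay randomizes the mesh, creates the HUD, and applies GameInstance level stats or saved data.
; ABP_Character events advance or end montage-section combos from buffered input, while Tick sphere-traces between trail sockets to apply damage.
; Interact messages both the overlapped target and every BPI_Interact actor; weapon swaps reattach between hand and holster sockets.
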(event `InputAxis|Turn Right / Left Mouse`
  (params (AxisValue :type "Float (single-precision)"))
  ;[1 1 1] 회전
  (`self.AddControllerYawInput` AxisValue))

(event `InputAxis|MoveForward / MoveBackward`
  (params (AxisValue :type "Float (single-precision)"))
  (bind (_returnvalue_roll _returnvalue_pitch _returnvalue_yaw) (`KismetMathLibrary.BreakRotator` (`self.GetControlRotation`)))
  ;[1 1 1] 이동
  (`self.AddMovementInput` (`KismetMathLibrary.GetForwardVector` (`KismetMathLibrary.MakeRotator` 0.0 0.0 _returnvalue_yaw)) AxisValue))

(event `InputAxis|LookUp / Down`
  (params (AxisValue :type "Float (single-precision)"))
  ;[1 1 1] 회전
  (`self.AddControllerPitchInput` AxisValue))

(event `InputAxis|MoveRight / MoveLeft`
  (params (AxisValue :type "Float (single-precision)"))
  (bind (_returnvalue_roll _returnvalue_pitch _returnvalue_yaw) (`KismetMathLibrary.BreakRotator` (`self.GetControlRotation`)))
  ;[1 1 1] 이동
  (`self.AddMovementInput` (`KismetMathLibrary.GetRightVector` (`KismetMathLibrary.MakeRotator` 0.0 0.0 _returnvalue_yaw)) AxisValue))

(event `InputAction|Jump`
  (params (Key :type "Key Structure"))
  ;[1 1 1] 점프
  (:`Pressed`
    (`self.Jump`))
  (:`Released`
    (`self.StopJumping`)))

(event `InputAction|Interact`
  (params (Key :type "Key Structure"))
  ;[1 1 1] 인터렉션 검증
  (:`Pressed`
    (`KismetSystemLibrary.PrintString` "Interact")
    (bind _outactors (`GameplayStatics.GetAllActorsWithInterface` "/Game/Blueprints/Interface/BPI_Interact.BPI_Interact_C"))
    (for _array_element _outactors
      (message `/Game/Blueprints/Interface/BPI_Interact.Interaction` _array_element))))

(event `self.InteractCollision.OnComponentBeginOverlap`
  (params (OverlappedComponent :type "PrimitiveComponent Object Reference") (OtherActor :type "Actor Object Reference") (OtherComp :type "PrimitiveComponent Object Reference") (OtherBodyIndex :type Integer) (bFromSweep :type Boolean) (SweepResult :type "HitResult Structure (by ref)"))
  ;[1 1 1] BPI 있는 액터인 경우 레퍼런스 등록
  (if (`KismetSystemLibrary.DoesImplementInterface` OtherActor)
    (set `self.Interact Target` OtherActor)))

(event `self.InteractCollision.OnComponentEndOverlap`
  (params (OverlappedComponent :type "PrimitiveComponent Object Reference") (OtherActor :type "Actor Object Reference") (OtherComp :type "PrimitiveComponent Object Reference") (OtherBodyIndex :type Integer))
  ;[1 1 1] 감지 해제 시 레퍼 날려주는 경우
  (if (== OtherActor (`self.Interact Target`))
    (set `self.Interact Target` null)))

(event `InputAction|Interact`
  (params (Key :type "Key Structure"))
  ;[1 1 1] 인터렉션 / Ref Valid인 경우 메시지 전달
  (:`Pressed`
    (`/Engine/EditorBlueprintResources/StandardMacros.IsValid` (`self.Interact Target`)
      (:`Is Valid`
        (message `/Game/Blueprints/Interface/BPI_Interact.Interaction` (`self.Interact Target`))))))

(event `self.ReceiveAnyDamage`
  (params (Damage :type "Float (single-precision)") (DamageType :type "DamageType Object Reference") (InstigatedBy :type "Controller Object Reference") (DamageCauser :type "Actor Object Reference"))
  (`self.Set HP` Damage)
  (if (`self.Is Dead`)
    (`/Engine/EditorBlueprintResources/StandardMacros.DoOnce` false :!label _label
      (:`Completed`
        (`KismetSystemLibrary.Delay` 5.0)
        (`self.Respawn`)
        (goto _label :!via `Reset`)))))

(event `InputAction|Attack`
  (params (Key :type "Key Structure"))
  ;[1 1 1] 무기
  (:`Pressed`
    (`/Engine/EditorBlueprintResources/StandardMacros.IsValid` (`self.CurrentWeapon`)
      (:`Is Valid`
        (`self.Attack`)))))

(event `InputAction|SwapWeapon1`
  (params (Key :type "Key Structure"))
  ;[1 1 1] 무기교체
  (:`Pressed`
    (`self.SwapWeapon1`)))

(event `InputAction|SwapWeapon2`
  (params (Key :type "Key Structure"))
  ;[1 1 1] 무기교체
  (:`Pressed`
    (`self.Swap Weapon 2`)))

(event `self.ReceiveBeginPlay`
  (bind _currentcharacterdata_level (break `/Game/Blueprints/DataTable/F_CharacterData` (`self.CurrentCharacterData`)))
  (`|ExecutionSequence`
    (:`then_0`
      ;[1 1 1] HP
      (`SkinnedMeshComponent.SetSkinnedAssetAndUpdate` (`self.Mesh`) (`|GetArrayItem` (`self.SK_Mesh_Arr`) (`KismetMathLibrary.RandomInteger` 17)) true)
      (bind _asbp_game_instance (cast `/Game/Blueprints/BP_GameInstance` (`GameplayStatics.GetGameInstance`)))
      (bind _character_data (`/Game/Blueprints/BP_GameInstance.GetCharacterData` _asbp_game_instance _currentcharacterdata_level))
      (bind _output_get (set `self.CurrentCharacterData` _character_data))
      (set `self.CurrentCharacterHP` (`.MaxHP_5_4FA2B7D04819608B548CFF901D8B4D07` (break `/Game/Blueprints/DataTable/F_CharacterData` _output_get))))
    (:`then_2`
      ;[1 1 1] 위젯
      (bind _returnvalue (`|CreateWidget` "/Game/Blueprints/UI/UMG_PlayerHUD.UMG_PlayerHUD_C" (`GameplayStatics.GetPlayerController` 0)))
      (`UserWidget.AddToViewport` _returnvalue 0)
      (`self.DisableInput` (`GameplayStatics.GetPlayerController` 0))
      (`KismetSystemLibrary.Delay` 2.5)
      (`self.EnableInput` (`GameplayStatics.GetPlayerController` 0)))
    (:`then_3`
      (bind _asbp_game_instance_2 (cast `/Game/Blueprints/BP_GameInstance` (`GameplayStatics.GetGameInstance`)))
      (`/Engine/EditorBlueprintResources/StandardMacros.IsValid` (`/Game/Blueprints/BP_GameInstance.LoadData` _asbp_game_instance_2)
        (:`Is Valid`
          (`self.Load Character Data`))
        (:`Is Not Valid`
          _))
      (`self.DisableInput` (`GameplayStatics.GetPlayerController` 0))
      ;[1 1 1] Attack
      (bind _asabp_character (cast `/Game/Blueprints/Character/ABP_Character` (`SkeletalMeshComponent.GetAnimInstance` (`self.Mesh`))))
      (bind _output_get_2 (set `self.AnimInstance` _asabp_character))
      ;;[1 1 1] OnNextAttackCheck
      (add `/Game/Blueprints/Character/ABP_Character.OnNextAttackCheck` _output_get_2 (delegate `OnNextAttackCheck`))
      (add `/Game/Blueprints/Character/ABP_Character.OnAttackMontageEnded` _output_get_2 (delegate `OnAttackMontageEnded`)))))

(event `OnAttackMontageEnded`
  ;[1 1 1] Attack
  (`self.AttackEndCombo`))

(event `OnNextAttackCheck`
  ;[1 1 1] Attack
  ;;[1 1 1] OnNextAttackCheck
  (if (`self.bIsComboInputOn`)
    (`self.AttackStartCombo`)
    (`/Game/Blueprints/Character/ABP_Character.JumpToAttackMontageSection` (`self.AnimInstance`) (`self.CurrentCombo`))
    (else
      (`AnimInstance.Montage_Stop` (`self.AnimInstance`) 0.25 null))))

(event `self.ReceiveTick`
  (params (DeltaSeconds :type "Float (single-precision)"))
  ;[1 1 1] Attack
  ;;[1 1 1] NS_AttackCheck
  (`self.AttackCheck`))

(fn `AddWeaponToSlot`
  (params (NewWeapon :type "/Game/Blueprints/Actors/BP_Weapon Object Reference"))
  ;[1 1 1] 웨폰 체크를 했는데 1번이 없으면 넣어주고 있으면 2번을 으로.
  (if (`KismetSystemLibrary.IsValid` (`self.WeaponSlot1`))
    (if (not (`KismetSystemLibrary.IsValid` (`self.WeaponSlot2`)))
      (bind _output_get (set `self.WeaponSlot2` (`local.NewWeapon`)))
      (`self.K2_AttachToComponent` (`self.WeaponSlot2`) (`self.Mesh`) "WeaponSlot2" "KeepRelative" "KeepRelative" "KeepRelative" true)
      (`self.K2_AttachToComponent` _output_get (`self.Mesh`) "WeaponSlot2" "KeepRelative" "KeepRelative" "KeepRelative" true))
    (else
      (bind _output_get_2 (set `self.WeaponSlot1` (`local.NewWeapon`)))
      (`self.K2_AttachToComponent` _output_get_2 (`self.Mesh`) "WeaponSlot1" "KeepRelative" "KeepRelative" "KeepRelative" true)
      (`self.K2_AttachToComponent` (`self.WeaponSlot1`) (`self.Mesh`) "WeaponSlot1" "KeepRelative" "KeepRelative" "KeepRelative" true))))

(fn `Attack`
  (if (`self.bIsAttacking`)
    ;[1 1 1] 콤보 입력 감지
    (set `self.bIsComboInputOn` true)
    (return)
    (else
      (`self.AttackStartCombo`)
      (`/Game/Blueprints/Character/ABP_Character.PlayAttackMontage` (`self.AnimInstance`))
      (`/Game/Blueprints/Character/ABP_Character.JumpToAttackMontageSection` (`self.AnimInstance`) (`self.CurrentCombo`))
      (set `self.bIsAttacking` true))))

(fn `AttackCheck`
  (bind (_currentcharacterdata_level _currentcharacterdata_maxhp _currentcharacterdata_attack) (break `/Game/Blueprints/DataTable/F_CharacterData` (`self.CurrentCharacterData`)))
  (bind _mesh (`self.Mesh`))
  (if (`self.bIsAttackCheck`)
    (bind _outhit (`KismetSystemLibrary.SphereTraceSingle` (`SceneComponent.GetSocketLocation` _mesh "Trail_Start") (`SceneComponent.GetSocketLocation` _mesh "Trail_End") 15.0 "TraceTypeQuery3" false (`self.HittedActor`) "ForDuration" true (struct :`R` 1.0 :`A` 1.0) (struct :`G` 1.0 :`A` 1.0) 1.0))
    (`KismetArrayLibrary.Array_AddUnique` (`self.HittedActor`) (`.HitActor` (`GameplayStatics.BreakHitResult` _outhit)))
    (`GameplayStatics.ApplyDamage` (`.HitActor` (`GameplayStatics.BreakHitResult` _outhit)) _currentcharacterdata_attack (`self.GetController`) self)
    (else
      (return))))

(fn `AttackEndCombo`
  (set `self.CanNextCombo` false)
  (set `self.bIsComboInputOn` false)
  (set `self.CurrentCombo` 0)
  (set `self.bIsAttacking` false))

(fn `AttackStartCombo`
  (locals (NewLocalVar_0 :type Boolean :default false))
  (if (`NavMovementComponent.IsFalling` (`self.CharacterMovement`))
    (set `self.CanNextCombo` false)
    (set `self.bIsComboInputOn` false)
    (set `self.CurrentCombo` 4)
    (else
      (set `self.CanNextCombo` true)
      (set `self.bIsComboInputOn` false)
      (set `self.CurrentCombo` (`KismetMathLibrary.Clamp` (+ (`self.CurrentCombo`) 1 0) 1 (`self.MaxCombo`))))))

(fn `CanGetWeapon`
  (returns (`Can Get Weapon` :type Boolean))
  (return (not (and (`KismetSystemLibrary.IsValid` (`self.WeaponSlot2`)) (`KismetSystemLibrary.IsValid` (`self.WeaponSlot1`))))))

(fn `Get Exp`
  (params (`New Exp` :type "Float (double-precision)"))
  (bind (_level _maxhp _attack _nextexp) (break `/Game/Blueprints/DataTable/F_CharacterData` (`self.CurrentCharacterData`)))
  (bind _output_get (set `self.CurrentExp` (+ `New Exp` (`self.CurrentExp`))))
  (if (>= _output_get _nextexp)
    ;[1 1 1] Level Up
    (`self.Level UP` (- _output_get _nextexp))))

(fn `Get Exp Ratio`
  (returns (ExpRatio :type "Float (double-precision)"))
  (return (/ (`self.CurrentExp`) (`.NextExp_11_5F28ED244584A332DE6F708175481E2C` (break `/Game/Blueprints/DataTable/F_CharacterData` (`self.CurrentCharacterData`))))))

(fn `Level UP`
  (params (remainExp :type "Float (double-precision)"))
  (locals (NewLocalVar_1 :type Integer))
  (`|ExecutionSequence`
    (:`then_0`
      (`KismetSystemLibrary.PrintString` "레벨업 이펙트"))
    (:`then_1`
      (bind _asbp_game_instance (cast `/Game/Blueprints/BP_GameInstance` (`GameplayStatics.GetGameInstance`)))
      (bind _character_data (`/Game/Blueprints/BP_GameInstance.GetCharacterData` _asbp_game_instance (+ (`.Level_3_CE2565F54F462CB07F8024B3F3E46510` (break `/Game/Blueprints/DataTable/F_CharacterData` (`self.CurrentCharacterData`))) 1))) ; 레벨업한 데이터를 가져오기
      (bind _output_get (set `self.CurrentCharacterData` _character_data))
      (set `self.CurrentCharacterHP` (`.MaxHP_5_4FA2B7D04819608B548CFF901D8B4D07` (break `/Game/Blueprints/DataTable/F_CharacterData` _output_get))) ; 레벨업 하면 체력 회복해주는거..
    )
    (:`then_2`
      (set `self.CurrentExp` remainExp))))

(fn `Load Character Data`
  (bind _asbp_game_instance (cast `/Game/Blueprints/BP_GameInstance` (`GameplayStatics.GetGameInstance`)))
  (bind _loaddata (`/Game/Blueprints/BP_GameInstance.LoadData` _asbp_game_instance))
  (bind _character_data (`/Game/Blueprints/BP_GameInstance.GetCharacterData` _asbp_game_instance (`/Game/Blueprints/BP_Savegame.CharacterLevel` _loaddata)))
  (bind _output_get (set `self.CurrentCharacterData` _character_data))
  (set `self.CurrentCharacterHP` (`/Game/Blueprints/BP_Savegame.CurrentHP` _loaddata))
  (bind _returnvalue (`|SpawnActorFromClass` (`/Game/Blueprints/BP_Savegame.Weapon1` _loaddata) (`KismetMathLibrary.MakeTransform` (0.0 0.0 0.0)) "AlwaysSpawn" "OverrideRootScale" null null))
  (`self.AddWeaponToSlot` _returnvalue)
  (bind _returnvalue_2 (`|SpawnActorFromClass` (`/Game/Blueprints/BP_Savegame.Weapon2` _loaddata) (`KismetMathLibrary.MakeTransform` (0.0 0.0 0.0)) "AlwaysSpawn" "OverrideRootScale" null null))
  (`self.AddWeaponToSlot` _returnvalue_2)
  (`self.K2_SetActorLocation` (`/Game/Blueprints/BP_Savegame.ActorLocation` _loaddata))
  (set `/Game/Blueprints/BP_GameInstance.LoadData` null _asbp_game_instance))

(fn `Respawn`
  (set `self.CurrentCharacterHP` (`.MaxHP_5_4FA2B7D04819608B548CFF901D8B4D07` (break `/Game/Blueprints/DataTable/F_CharacterData` (`self.CurrentCharacterData`))))
  (set `self.Is Dead` false)
  (`PrimitiveComponent.SetCollisionEnabled` (`self.CapsuleComponent`) "QueryAndPhysics")
  (`self.EnableInput` (`GameplayStatics.GetPlayerPawn` 0) (`GameplayStatics.GetPlayerController` 0)))

(fn `Set HP`
  (params (Damage :type "Float (double-precision)"))
  (bind _output_get (set `self.CurrentCharacterHP` (- (`self.CurrentCharacterHP`) Damage)))
  (`KismetSystemLibrary.PrintString` (`KismetStringLibrary.Concat_StrStr` "CurrentHP" (`KismetStringLibrary.Conv_DoubleToString` _output_get)))
  (if (<= (`self.CurrentCharacterHP`) 0.0)
    (set `self.Is Dead` true)
    (`PrimitiveComponent.SetCollisionEnabled` (`self.CapsuleComponent`) "NoCollision")
    (`self.DisableInput` (`GameplayStatics.GetPlayerPawn` 0) (`GameplayStatics.GetPlayerController` 0))
    (else
      (set `self.Is Dead` false))))

(fn `Set Weapon`
  (params (NewWeapon :type "/Game/Blueprints/Actors/BP_Weapon Object Reference")))

(fn `Swap Weapon 2`
  ;[1 1 1] 빈손 체크
  (`/Engine/EditorBlueprintResources/StandardMacros.IsValid` (`self.CurrentWeapon`)
    (:`Is Valid`
      ;[1 1 1] 2번 무기 장착한..
      (if (`KismetSystemLibrary.IsValid` (`self.WeaponSlot2`))
        (if (== (`self.CurrentWeapon`) (`self.WeaponSlot2`))
          ;[1 1 1] 2 장착
          (set `self.CurrentWeapon` null)
          (`self.K2_AttachToComponent` (`self.WeaponSlot2`) (`self.Mesh`) "WeaponSlot2" "SnapToTarget" "SnapToTarget" "SnapToTarget" true)
          (else
            ;[1 1 1] 현재 무기 2번 아님 / == 1번 무기 사용 중 -> 1번 무기 등으로 보냄, 2번 무기 착용
            (`self.K2_AttachToComponent` (`self.WeaponSlot1`) (`self.Mesh`) "WeaponSlot1" "SnapToTarget" "SnapToTarget" "SnapToTarget" true)
            (bind _output_get (set `self.CurrentWeapon` (`self.WeaponSlot2`)))
            (`self.K2_AttachToComponent` _output_get (`self.Mesh`) "R_Weapon" "SnapToTarget" "SnapToTarget" "SnapToTarget" true)))))
    (:`Is Not Valid`
      ;[1 1 1] 맨손인데 무기슬롯 2번에 무기가 있어서 / 2번 무기 장착
      (`/Engine/EditorBlueprintResources/StandardMacros.IsValid` (`self.WeaponSlot2`)
        (:`Is Valid`
          (bind _output_get_2 (set `self.CurrentWeapon` (`self.WeaponSlot2`)))
          (`self.K2_AttachToComponent` _output_get_2 (`self.Mesh`) "R_Weapon" "SnapToTarget" "SnapToTarget" "SnapToTarget" true))))))

(fn `SwapWeapon1`
  ;[1 1 1] 빈손 체크
  (`/Engine/EditorBlueprintResources/StandardMacros.IsValid` (`self.CurrentWeapon`)
    (:`Is Valid`
      ;[1 1 1] 장착한 무기가 있음
      (`/Engine/EditorBlueprintResources/StandardMacros.IsValid` (`self.WeaponSlot1`)
        (:`Is Valid`
          (if (== (`self.WeaponSlot1`) (`self.CurrentWeapon`))
            ;[1 1 1] True
            (set `self.CurrentWeapon` null)
            (`self.K2_AttachToComponent` (`self.WeaponSlot1`) (`self.Mesh`) "WeaponSlot1" "SnapToTarget" "SnapToTarget" "SnapToTarget" true)
            (else
              ;[1 1 1] 현재 무기가 1번이 아님/ == 2번 무기 사용중 -> 2번 무기 등으로 보내고, 1번 무기 착용
              (`self.K2_AttachToComponent` (`self.WeaponSlot2`) (`self.Mesh`) "WeaponSlot2" "SnapToTarget" "SnapToTarget" "SnapToTarget" true)
              (bind _output_get (set `self.CurrentWeapon` (`self.WeaponSlot1`)))
              (`self.K2_AttachToComponent` _output_get (`self.Mesh`) "R_Weapon" "SnapToTarget" "SnapToTarget" "SnapToTarget" true))))))
    (:`Is Not Valid`
      ;[1 1 1] 맨손인데 무기슬롯 1번에 무기가 있어서 / 1번 무기 장착
      (`/Engine/EditorBlueprintResources/StandardMacros.IsValid` (`self.WeaponSlot1`)
        (:`Is Valid`
          (bind _output_get_2 (set `self.CurrentWeapon` (`self.WeaponSlot1`)))
          (`self.K2_AttachToComponent` _output_get_2 (`self.Mesh`) "R_Weapon" "SnapToTarget" "SnapToTarget" "SnapToTarget" true))))))

(fn `UserConstructionScript`)