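; Gate actor whose door swings open away from the local player's pawn on entering its trigger box, then closes on exit or after a short timer.
; CheckDir takes the dot product of the pawn-to-gate vector and the gate's forward vector to pick the swing direction.
; Separate open and close timelines lerp the door's relative yaw from its current angle, each stopping the other to handle mid-swing reversals.
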(event `self.Box.OnComponentBeginOverlap`
  (params (OverlappedComponent :type "PrimitiveComponent Object Reference") (OtherActor :type "Actor Object Reference") (OtherComp :type "PrimitiveComponent Object Reference") (OtherBodyIndex :type Integer) (bFromSweep :type Boolean) (SweepResult :type "HitResult Structure (by ref)"))
  (bind _returnvalue (`GameplayStatics.GetPlayerController` 0))
  (bind (_relativerotation_roll _relativerotation_pitch _relativerotation_yaw) (`KismetMathLibrary.BreakRotator` (`SceneComponent.RelativeRotation` (`self.SM_Door`))))
  ;[1 1 1] 트리거 조건 예외처리(내 캐릭터인 경우만)
  (`/Engine/EditorBlueprintResources/StandardMacros.IsValid` _returnvalue
    (:`Is Valid`
      (if (== OtherActor (`Controller.K2_GetPawn` _returnvalue))
        (`self.DoorClose_Stop`)
        (`self.CheckDir`)
        (set `self.CurrentYaw` _relativerotation_yaw)
        (set `self.TargetYaw` 90.0)
        ;[1 1 1] 1초
        (bind (_direction _alpha) (`Timeline|TL_DoorOpen` :!via `PlayFromStart` :!label _label)
          (:`Update`
            (`self.Open_Dynamic Gate` _alpha))
          (:`Finished`
            ;[1 1 1] 닫히는 기능 추가
            (`KismetSystemLibrary.K2_SetTimerDelegate` (delegate `CloseDoorByTimer`) 3.0)))))))

(event `DoorOpen_Stop`
  (goto _label :!via `Stop`))

(event `CloseDoorByTimer`
  (bind (_relativerotation_roll _relativerotation_pitch _relativerotation_yaw) (`KismetMathLibrary.BreakRotator` (`SceneComponent.RelativeRotation` (`self.SM_Door`))))
  (`self.DoorOpen_Stop` :!label _label_2)
  (set `self.CurrentYaw` _relativerotation_yaw)
  (set `self.TargetYaw` 0.0)
  (bind (_direction _alpha) (`Timeline|TL_DoorClose` :!via `PlayFromStart` :!label _label_3)
    (:`Update`
      (`self.Close_Dynamic Gate` _alpha))))

(event `self.Box.OnComponentEndOverlap`
  (params (OverlappedComponent :type "PrimitiveComponent Object Reference") (OtherActor :type "Actor Object Reference") (OtherComp :type "PrimitiveComponent Object Reference") (OtherBodyIndex :type Integer))
  (bind _returnvalue (`GameplayStatics.GetPlayerController` 0))
  (`/Engine/EditorBlueprintResources/StandardMacros.IsValid` _returnvalue
    (:`Is Valid`
      (if (== OtherActor (`Controller.K2_GetPawn` _returnvalue))
        (goto _label_2)))))

(event `DoorClose_Stop`
  (goto _label_3 :!via `Stop`))

(fn `CheckDir`
  ;[1 1 1] 양수 정면 음수 후면
  (if (> (`KismetMathLibrary.Dot_VectorVector` (`KismetMathLibrary.Normal` (- (`self.K2_GetActorLocation`) (`self.K2_GetActorLocation` (`Controller.K2_GetPawn` (`GameplayStatics.GetPlayerController` 0))))) (`self.GetActorForwardVector`)) 0.0)
    (set `self.Dir` 1.0)
    (else
      (set `self.Dir` -1.0))))

(fn `Close_Dynamic Gate`
  (params (Alpha :type "Float (double-precision)"))
  (locals (Direction :type "Vector Structure" :default (0.0 0.0 0.0)) (Loc_Degree :type "Float (double-precision)" :default 90.0))
  (`SceneComponent.K2_SetRelativeRotation` (`self.SM_Door`) (`KismetMathLibrary.MakeRotator` 0.0 0.0 (`KismetMathLibrary.Lerp` (`self.TargetYaw`) (`self.CurrentYaw`) Alpha)) false false))

(fn `Open_Dynamic Gate`
  (params (Alpha :type "Float (double-precision)"))
  (locals (Direction :type "Vector Structure" :default (0.0 0.0 0.0)) (Loc_Degree :type "Float (double-precision)" :default 90.0))
  (`SceneComponent.K2_SetRelativeRotation` (`self.SM_Door`) (`KismetMathLibrary.MakeRotator` 0.0 0.0 (`KismetMathLibrary.Lerp` (`self.CurrentYaw`) (* (`self.Dir`) (`self.TargetYaw`)) Alpha)) false false))

(fn `UserConstructionScript`)