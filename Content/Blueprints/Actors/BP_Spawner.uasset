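; BP_Spawner is a spawner actor that keeps a population of actors, apparently bears, inside a box volume up to a maximum count.
; BeginPlay spawns the initial batch at random points in the box and starts a looping timer that adds one actor whenever the list is short.
; Each spawn receives a ParentSpawner reference, and RemoveDeadBear drops dead ones from the tracked list so they get replaced.
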(event `RemoveDeadBear`
  (params (DeadBear :type "/Game/Blueprints/Bear/BP_Bear Object Reference"))
  (`KismetArrayLibrary.Array_RemoveItem` (`self.SpawnedActorList`) DeadBear)
  (`KismetSystemLibrary.PrintString` "Bear Dead"))

(event `self.ReceiveBeginPlay`
  (for _ (range (`self.MaxSpawned`))
    (`self.SpawnActorByClass`)
    (`KismetSystemLibrary.K2_SetTimerDelegate` (delegate `CheckList`) 5.0 true) ; 5초마다 한 마리씩 리스폰
  ))

(event `CheckList`
  (if (< (`KismetArrayLibrary.Array_Length` (`self.SpawnedActorList`)) (`self.MaxSpawned`))
    (`KismetSystemLibrary.PrintString` "Timer Spawn")
    (`self.SpawnActorByClass`)))

(fn `SpawnActorByClass`
  (returns (ReturnValue :type "/Game/Blueprints/Bear/BP_Bear Object Reference"))
  (bind (_origin _boxextent) (`KismetSystemLibrary.GetComponentBounds` (`self.Box`)))
  (bind _returnvalue (`|SpawnActorFromClass` (`self.Spawn Class`) (`KismetMathLibrary.MakeTransform` (`KismetMathLibrary.RandomPointInBoundingBox` _origin _boxextent)) "AdjustIfPossibleButAlwaysSpawn" "OverrideRootScale" null null))
  (set `/Game/Blueprints/Bear/BP_Bear.ParentSpawner` self _returnvalue)
  (`KismetArrayLibrary.Array_Add` (`self.SpawnedActorList`) _returnvalue)
  (return _returnvalue))

(fn `UserConstructionScript`)