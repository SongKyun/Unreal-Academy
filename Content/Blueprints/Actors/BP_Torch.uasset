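; BP_Torch is a torch actor whose flame particle system can be switched on and off.
; The Interaction event toggles the ParticleSystem's active state, while OffTorch forces it off.
; The overlap events do nothing, though end overlap still branches on a BP_Character class check.
; A disconnected older toggle with debug prints remains in the graph.
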(event `/Game/Blueprints/Interface/BPI_Interact.Interaction`
  ;[1 1 1] on/off 행위
  (if (`ActorComponent.IsActive` (`self.ParticleSystem`))
    (`ActorComponent.SetActive` (`self.ParticleSystem`) false false)
    (else
      (`ActorComponent.SetActive` (`self.ParticleSystem`) true false))))

(event `self.ReceiveActorBeginOverlap`
  (params (OtherActor :type "Actor Object Reference")))

(event `OffTorch`
  (`ActorComponent.SetActive` (`self.ParticleSystem`) false false))

(event `self.ReceiveActorEndOverlap`
  (params (OtherActor :type "Actor Object Reference"))
  (if (== (`GameplayStatics.GetObjectClass` OtherActor) "/Game/Blueprints/Character/BP_Character.BP_Character_C")
    _))

(fn `UserConstructionScript`)