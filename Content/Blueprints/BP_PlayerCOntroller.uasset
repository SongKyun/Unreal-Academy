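; Player controller that opens the in-game menu and plays an intro camera effect when play begins.
; The Menu input creates UMG_Menu on first press, caches it, and re-adds it at a high Z-order on later presses if it is off-screen, without toggling it closed.
; BeginPlay sets game-only input, fades the camera in from opaque, then starts a strong world-space camera shake after the fade.
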(event `InputAction|Menu`
  (params (Key :type "Key Structure"))
  (:`Pressed`
    (`/Engine/EditorBlueprintResources/StandardMacros.IsValid` (`self.WB_Menu`)
      (:`Is Valid`
        (if (not (`Widget.IsInViewport` (`self.WB_Menu`)))
          (`UserWidget.AddToViewport` (`self.WB_Menu`) 99)))
      (:`Is Not Valid`
        (bind _returnvalue (`|CreateWidget` "/Game/Blueprints/UI/UMG_Menu.UMG_Menu_C" (`GameplayStatics.GetPlayerController` 0)))
        (bind _output_get (set `self.WB_Menu` _returnvalue)) ; 캐싱
        (`UserWidget.AddToViewport` _output_get 99)))))

(event `self.ReceiveBeginPlay`
  (bind _playercameramanager (`self.PlayerCameraManager`))
  (`WidgetBlueprintLibrary.SetInputMode_GameOnly` self)
  (`PlayerCameraManager.StartCameraFade` :`self` _playercameramanager :`FromAlpha` 1.0 :`Duration` 2.5)
  (`KismetSystemLibrary.Delay` 2.5)
  (`PlayerCameraManager.StartCameraShake` :`self` _playercameramanager :`ShakeClass` "/Game/Blueprints/BP_CameraShacke.BP_CameraShacke_C" :`Scale` 10.0 :`PlaySpace` "World"))

(fn `UserConstructionScript`)