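; Enemy bear character that chases a seen player through its AI Blackboard, with stats loaded from DT_BearData.
; A state dispatcher sets walk speed per state.
; The attack collision gathers overlapped actors and damages them when switched off.
; Damage flashes the mesh; at zero HP the AI logic stops, the bear dissolves, awards EXP to the killer, notifies its spawner and is destroyed.
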(event `self.ReceiveBeginPlay`
  (bind _returnvalue (`WidgetComponent.GetWidget` (`self.Healthbar`)))
  ;[1 1 1] 이벤트 디스패처를 사용해 모드에 따른 이동속도 설정
  (`|ExecutionSequence`
    (:`then_0`
      (add `self.OnStateChanged` (delegate `OnStateChanged_Event`)))
    (:`then_1`
      (`KismetSystemLibrary.PrintString` (`KismetSystemLibrary.GetDisplayName` _returnvalue))
      (bind _asumg_enemy_healthbar (cast `/Game/Blueprints/UI/UMG_EnemyHealthbar` _returnvalue))
      (set `/Game/Blueprints/UI/UMG_EnemyHealthbar.Owner` self _asumg_enemy_healthbar))))

(event `OnStateChanged_Event`
  (bind _charactermovement (`self.CharacterMovement`))
  ;[1 1 1] 이벤트 디스패처를 사용해 모드에 따른 이동속도 설정
  (switch `/Game/Blueprints/Bear/Enemy_Bear/E_BearState` (`self.State`)
    (:`NewEnumerator0`
      (set `CharacterMovementComponent.MaxWalkSpeed` 200.0 _charactermovement))
    (:`NewEnumerator1`
      (set `CharacterMovementComponent.MaxWalkSpeed` 400.0 _charactermovement))
    (:`NewEnumerator2`
      (set `CharacterMovementComponent.MaxWalkSpeed` 0.0 _charactermovement :!label _label))
    (:`NewEnumerator3`
      (goto _label))))

(event `self.PawnSensing.OnSeePawn`
  (params (Pawn :type "Pawn Object Reference"))
  (bind _asbp_character (cast `/Game/Blueprints/Character/BP_Character` Pawn))
  (`BlackboardComponent.SetValueAsObject` (`AIBlueprintHelperLibrary.GetBlackboard` (`self.GetController`)) "TargetPlayer" _asbp_character)
  (bind _output_get (set `self.State` "NewEnumerator1"))
  (`BlackboardComponent.SetValueAsEnum` (`AIBlueprintHelperLibrary.GetBlackboard` (`self.GetController`)) "BearState" _output_get)
  (`self.OnStateChanged`))

(event `self.AttackCollision.OnComponentBeginOverlap`
  (params (OverlappedComponent :type "PrimitiveComponent Object Reference") (OtherActor :type "Actor Object Reference") (OtherComp :type "PrimitiveComponent Object Reference") (OtherBodyIndex :type Integer) (bFromSweep :type Boolean) (SweepResult :type "HitResult Structure (by ref)"))
  (`KismetArrayLibrary.Array_AddUnique` (`self.HittedActor`) OtherActor))

(event `self.ReceiveAnyDamage`
  (params (Damage :type "Float (single-precision)") (DamageType :type "DamageType Object Reference") (InstigatedBy :type "Controller Object Reference") (DamageCauser :type "Actor Object Reference"))
  (`self.Set Health` Damage)
  (`self.HittedEffect`)
  (set `self.DamageCauser` DamageCauser))

(event `HittedEffect`
  (bind (_direction _color) (`Timeline|TL_HittedEffect` :!via `PlayFromStart`)
    (:`Update`
      (`MeshComponent.SetVectorParameterValueOnMaterials` (`self.Mesh`) "HittedColor" (`KismetMathLibrary.MakeVector` _color)))))

(event `DissolveIntensity`
  (bind (_currentstat_level _currentstat_maxhp _currentstat_attack _currentstat_dropexp) (break `/Game/Blueprints/DataTable/Bear_DataTable/F_BearData` (`self.CurrentStat`)))
  (bind _parentspawner (`self.ParentSpawner`))
  (bind (_direction _v) (`Timeline|TL_V` :!via `PlayFromStart`)
    (:`Update`
      (`MeshComponent.SetScalarParameterValueOnMaterials` (`self.Mesh`) "DissolveIntensity" _v))
    (:`Finished`
      (`|ExecutionSequence`
        (:`then_0`
          (`/Engine/EditorBlueprintResources/StandardMacros.IsValid` (`self.DamageCauser`)
            (:`Is Valid`
              (bind _asbp_character (cast `/Game/Blueprints/Character/BP_Character` (`self.DamageCauser`))
                (:`then`
                  (`/Game/Blueprints/Character/BP_Character.Get Exp` _asbp_character _currentstat_dropexp))
                (:`CastFailed`
                  _)))
            (:`Is Not Valid`
              _))
          (`/Engine/EditorBlueprintResources/StandardMacros.IsValid` _parentspawner
            (:`Is Valid`
              (`/Game/Blueprints/Actors/BP_Spawner.RemoveDeadBear` _parentspawner self))
            (:`Is Not Valid`
              _))
          (`self.K2_DestroyActor`))
        (:`then_1`
          (`self.K2_DestroyActor`))))))

(fn `GetHealthRatio`
  (returns (HealthPercent :type "Float (double-precision)"))
  (return (/ (`self.Current HP`) (`.MaxHp_7_0134CC874152660CF142BAA0F67EA823` (break `/Game/Blueprints/DataTable/Bear_DataTable/F_BearData` (`self.CurrentStat`))))))

(fn `Set Health`
  (params (`New Damage` :type "Float (double-precision)"))
  (bind _output_get (set `self.Current HP` (- (`self.Current HP`) `New Damage`)))
  (if (<= _output_get 0.0)
    (set `self.State` "NewEnumerator3")
    (`BrainComponent.StopLogic` (`AIController.BrainComponent` (`AIBlueprintHelperLibrary.GetAIController` self)) "")
    (`PrimitiveComponent.SetCollisionEnabled` (`self.CapsuleComponent`) "NoCollision")
    (`self.DissolveIntensity`) ; 커스텀 이벤트를 불러주는게 있어야 한다.
  ))

(fn `SetAttackCollision`
  (params (`Is Enable` :type Boolean))
  (if `Is Enable`
    (`PrimitiveComponent.SetCollisionEnabled` (`self.AttackCollision`) "QueryOnly")
    (else
      (`PrimitiveComponent.SetCollisionEnabled` (`self.AttackCollision`) "NoCollision")
      (for _array_element (`self.HittedActor`)
        (`GameplayStatics.ApplyDamage` _array_element (`self.AttackDamage`) (`self.GetController`) self))
      (`KismetArrayLibrary.Array_Clear` (`self.HittedActor`)))))

(fn `UserConstructionScript`
  (`PrimitiveComponent.SetCollisionEnabled` (`self.AttackCollision`) "NoCollision")
  (bind _returnvalue (`|GetDataTableRow` "/Game/Blueprints/DataTable/Bear_DataTable/DT_BearData.DT_BearData" "1")
    (:`then`
      (bind _output_get (set `self.CurrentStat` _returnvalue)) ; 곰돌이의 현재 스텟
      (set `self.Current HP` (`.MaxHp_7_0134CC874152660CF142BAA0F67EA823` (break `/Game/Blueprints/DataTable/Bear_DataTable/F_BearData` _output_get))) ; 이거 왜 해주지? 체력을 설정
    )))